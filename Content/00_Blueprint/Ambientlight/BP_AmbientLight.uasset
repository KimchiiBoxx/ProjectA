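; BP_AmbientLight is an ambient light actor with a sphere whose emissive color can be switched between presets.
; On BeginPlay it creates a dynamic material instance from MI_AmbientLight on the sphere and stores it.
; Custom events for white, blue, red, yellow and green each set that instance's Emissive Color parameter.
; RedColor and YellowColor currently apply the same pinkish value.
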(event Custom|White%20Color
  (Rendering|Material|SetVectorParameterValue (Variables|Default|GetDynamicAmbientMaterial) "Emissive Color" "(R=0.351295,G=0.383873,B=0.526042,A=1.000000)" :!class /Script/Engine.MaterialInstanceDynamic))

(event Custom|Blue%20Color
  (Rendering|Material|SetVectorParameterValue (Variables|Default|GetDynamicAmbientMaterial) "Emissive Color" "(R=0.068495,G=0.135482,B=0.526042,A=1.000000)" :!class /Script/Engine.MaterialInstanceDynamic))

(event Custom|Red%20Color
  (Rendering|Material|SetVectorParameterValue (Variables|Default|GetDynamicAmbientMaterial) "Emissive Color" (Utilities|Struct|MakeLinearColor 0.913099 0.433266 0.543313 1.0) :!class /Script/Engine.MaterialInstanceDynamic))

(event Custom|Yellow%20Color
  (Rendering|Material|SetVectorParameterValue (Variables|Default|GetDynamicAmbientMaterial) "Emissive Color" (Utilities|Struct|MakeLinearColor 0.913099 0.433266 0.543313 1.0) :!class /Script/Engine.MaterialInstanceDynamic))

(event Custom|Green%20Color
  (Rendering|Material|SetVectorParameterValue (Variables|Default|GetDynamicAmbientMaterial) "Emissive Color" (Utilities|Struct|MakeLinearColor 0.548921 0.913099 0.665679 1.0) :!class /Script/Engine.MaterialInstanceDynamic))

(event EventBeginPlay
  (bind _returnvalue (Rendering|Material|CreateDynamicMaterialInstance (Variables|Default|GetSphere) 0 "/Game/02_Material/MI_AmbientLight.MI_AmbientLight" "None" :!class /Script/Engine.PrimitiveComponent))
  (Variables|Default|SetDynamicAmbientMaterial _returnvalue))

(fn ConstructionScript)