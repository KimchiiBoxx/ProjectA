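; Audi car indicator actor that brightens and dims a red light as the third-person character enters and leaves its overlap area.
; Begin and end overlap both call IndicatorSignal, which lazily creates and caches a dynamic material instance on the Cylinder's red light slot.
; A FlipFlop then alternates the emissive value between bright and dim, so the state follows call order rather than the overlap type.
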(event Custom|Indicator%20Signal
  ;[1 1 1] Near Car Signal
  ;;[1 1 1] Check Dynamic Material present (not present = true)
  (if (== (Variables|Default|GetDynamicMaterialIndicator) 0)
    ;;[1 1 1] Create Dynamic Material Instance
    (bind _returnvalue (Rendering|Material|CreateDynamicMaterialInstance (Variables|Default|GetCylinder) 2 "/Game/02_Material/MI_AUDI_RedLight.MI_AUDI_RedLight" "None" :!class /Script/Engine.PrimitiveComponent))
    (Variables|Default|SetDynamicMaterialIndicator _returnvalue))
  ;;[1 1 1] Switch
  (Utilities|FlowControl|FlipFlop
    (:A
      (Rendering|Material|SetScalarParameterValue (Variables|Default|GetDynamicMaterialIndicator) "Emissive Value" 1e+03 :!class /Script/Engine.MaterialInstanceDynamic))
    (:B
      (Rendering|Material|SetScalarParameterValue (Variables|Default|GetDynamicMaterialIndicator) "Emissive Value" 1.0 :!class /Script/Engine.MaterialInstanceDynamic))))

(event Collision|EventActorEndOverlap
  (params (OtherActor :type Actor%20Object%20Reference))
  ;[1 1 1] Near Car Signal
  (Utilities|Casting|CastToBP_ThirdPersonCharacter OtherActor)
  (CallFunction|IndicatorSignal))

(event Collision|EventActorBeginOverlap
  (params (OtherActor :type Actor%20Object%20Reference))
  ;[1 1 1] Near Car Signal
  (Utilities|Casting|CastToBP_ThirdPersonCharacter OtherActor)
  (CallFunction|IndicatorSignal))

(fn ConstructionScript)