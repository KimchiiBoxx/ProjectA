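; BP_Signal is an Audi car actor that reacts to the player approaching and lets them enter its interior level.
; Player overlap begin and end both call AudiSignal, which lazily creates a dynamic red-light material and uses a FlipFlop to toggle its emissive glow.
; A separate EnterCarTrigger shows or hides the WBIndicator widget.
; EnterCar saves the character's name to the Game Instance, then opens Map_PrototypInterior.
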(event OnComponentBeginOverlap(EnterCarTrigger)
  (params (OverlappedComponent :type Primitive%20Component%20Object%20Reference) (OtherActor :type Actor%20Object%20Reference) (OtherComp :type Primitive%20Component%20Object%20Reference) (OtherBodyIndex :type Integer) (bFromSweep :type Boolean) (SweepResult :type Hit%20Result%20Structure%20%28by%20ref%29))
  (Rendering|SetVisibility (Variables|Default|GetWB_Indicator) true false))

(event OnComponentEndOverlap(EnterCarTrigger)
  (params (OverlappedComponent :type Primitive%20Component%20Object%20Reference) (OtherActor :type Actor%20Object%20Reference) (OtherComp :type Primitive%20Component%20Object%20Reference) (OtherBodyIndex :type Integer))
  (Rendering|SetVisibility (Variables|Default|GetWB_Indicator) false false))

(event Custom|AudiSignal
  ;[1 1 1] Near Car Signal
  ;;[1 1 1] Check Dynamic Material present (not present = true)
  (if (== (Variables|Default|GetDynamicMaterial) 0)
    ;;[1 1 1] Create Dynamic Material Instance
    (bind _returnvalue (Rendering|Material|CreateDynamicMaterialInstance (Variables|Default|GetStaticMesh) 0 "/Game/02_Material/MI_AUDI_RedLight.MI_AUDI_RedLight" "None" :!class /Script/Engine.PrimitiveComponent))
    (Variables|Default|SetDynamicMaterial _returnvalue))
  ;;[1 1 1] Switch
  (Utilities|FlowControl|FlipFlop
    (:A
      (Rendering|Material|SetScalarParameterValue (Variables|Default|GetDynamicMaterial) "Emissive Value" 1e+02 :!class /Script/Engine.MaterialInstanceDynamic))
    (:B
      (Rendering|Material|SetScalarParameterValue (Variables|Default|GetDynamicMaterial) "Emissive Value" 1.0 :!class /Script/Engine.MaterialInstanceDynamic))))

(event EventEnterCar
  ;[1 1 1] Save Name Character to Game Instance before change level
  (bind _asbpi_name_instance (Utilities|Casting|CastToBPI_NameInstance (Game|GetGameInstance)))
  (bind _asbp_third_person_character (Utilities|Casting|CastToBP_ThirdPersonCharacter (Game|GetPlayerCharacter 0)))
  (Variables|/Game/00_Blueprint/BPI_NameInstance.BPI_NameInstance_C|SetPlayerNameInstance _asbpi_name_instance (Variables|/Game/ThirdPerson/Blueprints/BP_ThirdPersonCharacter.BP_ThirdPersonCharacter_C|GetName%20Character _asbp_third_person_character))
  (Game|OpenLevel(byName) "Map_PrototypInterior"))

(event Collision|EventActorBeginOverlap
  (params (OtherActor :type Actor%20Object%20Reference))
  ;[1 1 1] Near Car Signal
  (Utilities|Casting|CastToBP_ThirdPersonCharacter OtherActor)
  (CallFunction|AudiSignal))

(event Collision|EventActorEndOverlap
  (params (OtherActor :type Actor%20Object%20Reference))
  ;[1 1 1] Near Car Signal
  (Utilities|Casting|CastToBP_ThirdPersonCharacter OtherActor)
  (CallFunction|AudiSignal))

(fn ConstructionScript)